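; BP_Player is the runner game's player Blueprint, which moves forward automatically until it dies.
; Axis events add movement along control-yaw directions, with forward fixed at full scale and sideways following input.
; Death clears GameMode_Runner's timer, stops forward movement, ragdolls the mesh with a heavy mass override, then reloads the GamePlay level after a short delay.
; The Q key quits the game.
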(event Custom|Death
  (bind _returnvalue (Game|GetPlayerCharacter 0))
  (bind _mesh (Variables|/Script/Engine.Character|GetMesh _returnvalue))
  (bind _asgame_mode_runner (Utilities|Casting|CastToGameMode_Runner (Game|GetGameMode)))
  (Utilities|Time|ClearandInvalidateTimerbyHandle (Variables|/Game/Runner_Game/Game_Mode/GameMode_Runner.GameMode_Runner_C|GetTimer%20Handler _asgame_mode_runner))
  (Variables|Default|SetIs%20Player%20Dead true)
  (Components|SkinnedMesh|SetPhysicsAsset _mesh "/Game/Mannequin/Character/Mesh/SK_Mannequin_PhysicsAsset.SK_Mannequin_PhysicsAsset" false)
  (Physics|SetSimulatePhysics _mesh true)
  (Class|PrimitiveComponent|SetMassOverrideinKg _mesh "None" 1e+03 true)
  (Utilities|FlowControl|Delay 2.0)
  (Game|OpenLevel(byName) "GamePlay"))

(event Input|AxisEvents|InputAxisMoveRight
  (params (AxisValue :type Float%20%28single-precision%29))
  (Pawn|Input|AddMovementInput (Math|Vector|GetRightVector (Math|Rotator|MakeRotator 0.0 0.0 (.Yaw (Math|Rotator|BreakRotator (Pawn|GetControlRotation :!class /Script/Engine.Pawn))))) AxisValue false))

(event Input|AxisEvents|InputAxisMoveForward
  (params (AxisValue :type Float%20%28single-precision%29))
  (if (not (Variables|Default|GetIs%20Player%20Dead))
    (Pawn|Input|AddMovementInput (Math|Vector|GetForwardVector (Math|Rotator|MakeRotator 0.0 0.0 (.Yaw (Math|Rotator|BreakRotator (Pawn|GetControlRotation :!class /Script/Engine.Pawn))))) 1.0 false)))

(event Input|KeyboardEvents|Q
  (params (Key :type Key%20Structure :default "None"))
  (:Pressed
    (Game|QuitGame 0 "Quit" false)))

(fn ConstructionScript)