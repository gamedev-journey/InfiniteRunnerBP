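; BP_LevelFloor is a floor segment for a runner game that carries one random obstacle and removes itself once passed.
; Its construction script adds a child actor of one of three obstacle classes at the right, left or center spawn point, both picked randomly.
; An EndTrigger overlap tells GameMode_Runner to AddMap, then destroys the segment after a short delay.
; GetAttachTransform exposes the AttachPoint's world transform.
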(event OnComponentBeginOverlap(EndTrigger)
  (params (OverlappedComponent :type Primitive%20Component%20Object%20Reference) (OtherActor :type Actor%20Object%20Reference) (OtherComp :type Primitive%20Component%20Object%20Reference) (OtherBodyIndex :type Integer) (bFromSweep :type Boolean) (SweepResult :type Hit%20Result%20Structure%20%28by%20ref%29))
  (bind _asgame_mode_runner (Utilities|Casting|CastToGameMode_Runner (Game|GetGameMode)))
  (Default|AddMap _asgame_mode_runner)
  (Utilities|FlowControl|Delay 0.5)
  (Actor|DestroyActor))

(event EventBeginPlay)

(event Collision|EventActorBeginOverlap
  (params (OtherActor :type Actor%20Object%20Reference)))

(event EventTick
  (params (DeltaSeconds :type Float%20%28single-precision%29)))

(fn ConstructionScript
  (CallFunction|SetSpawnPoints)
  (CallFunction|SetObstacles)
  (CallFunction|SpawnObstacles))

(fn SetSpawnPoints
  (Variables|Default|SetSpawn%20Points (Utilities|Array|MakeArray (Transformation|GetRelativeTransform (Variables|Default|GetSpawn%20R)) (Transformation|GetRelativeTransform (Variables|Default|GetSpawn%20L)) (Transformation|GetRelativeTransform (Variables|Default|GetSpawn%20Center)))))

(fn SetObstacles
  (Variables|Default|SetObstacles (Utilities|Array|MakeArray "/Game/Runner_Game/Game_Items/BP_Obstacle1.BP_Obstacle1_C" "/Game/Runner_Game/Game_Items/BP_Obstacle2.BP_Obstacle2_C" "/Game/Runner_Game/Game_Items/BP_Obstacle3.BP_Obstacle3_C")))

(fn SpawnObstacles
  (bind _obstacles (Variables|Default|GetObstacles))
  (bind _spawn_points (Variables|Default|GetSpawn%20Points))
  (bind _returnvalue (AddComponent|AddChildActorComponent false (Utilities|Array|Get(acopy) _spawn_points (Math|Random|RandomIntegerinRange 0 (Utilities|Array|LastIndex _spawn_points)))))
  (ChildActorComponent|SetChildActorClass _returnvalue (Utilities|Array|Get(acopy) _obstacles (Math|Random|RandomIntegerinRange 0 (Utilities|Array|LastIndex _obstacles)))))

(fn GetAttachTransform
  (return (Transformation|GetWorldTransform (Variables|Default|GetAttach%20Point))))